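; Generic AI controller that runs BT_AI and feeds it perception results for chasing and investigating targets.
; Each perception update goes to sight and hearing handlers that write to the blackboard.
; Successful sight sets TargetActor, while any non-sight stimulus clears it; losing sight alone leaves it unchanged.
; Hearing stores the stimulus location as InvestigationLocation and calls InvestigationIcon on the controlled BP_Character_AI.
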(event OnTargetPerceptionUpdated(AIPerception)
  (params (Actor :type Actor%20Object%20Reference) (Stimulus :type AI%20Stimulus%20Structure))
  ;[1 1 1] Detect, Chase and Investigate Target
  (CallFunction|SightDetection Actor Stimulus)
  (CallFunction|HearingDetection Actor Stimulus))

(event EventBeginPlay
  (AI|RunBehaviorTree "/Game/_mystuff/Characters/AI/BT_AI.BT_AI"))

(fn ConstructionScript)

(fn SightDetection
  (params (Actor :type Actor%20Object%20Reference) (Stimulus :type AI%20Stimulus%20Structure))
  (bind _returnvalue (Class|AIPerceptionSystem|GetSenseClassforStimulus Stimulus))
  (if (== _returnvalue "/Script/AIModule.AISense_Sight")
    (if (.bSuccessfullySensed (Utilities|Struct|BreakAIStimulus Stimulus))
      (AI|Components|Blackboard|SetValueasObject (AI|GetBlackboard 0) (Utilities|Name|MakeLiteralName "TargetActor") Actor))
    (else
      (AI|Components|Blackboard|SetValueasObject (AI|GetBlackboard 0) (Utilities|Name|MakeLiteralName "TargetActor") 0))))

(fn HearingDetection
  (params (Actor :type Actor%20Object%20Reference) (Stimulus :type AI%20Stimulus%20Structure))
  (bind _returnvalue (Class|AIPerceptionSystem|GetSenseClassforStimulus Stimulus))
  (if (== _returnvalue "/Script/AIModule.AISense_Hearing")
    (AI|Components|Blackboard|SetValueasVector (AI|GetBlackboard 0) (Utilities|Name|MakeLiteralName "InvestigationLocation") (.StimulusLocation (Utilities|Struct|BreakAIStimulus Stimulus)))
    (bind _asbp_character_ai (Utilities|Casting|CastToBP_Character_AI (Pawn|GetControlledPawn)))
    (Default|InvestigationIcon _asbp_character_ai)))