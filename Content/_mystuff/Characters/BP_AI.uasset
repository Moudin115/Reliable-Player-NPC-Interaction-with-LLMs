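; Conversational NPC character that chats with the player by text or voice, faces them, and can open a shop.
; Typed or speech-recognized input goes via VaRest to OpenAI with a persona, time and memory prompt.
; Replies fill the chat widget, trigger the shop by tag, and play as ElevenLabs speech.
; Closing chat requests a tagged memory summary, but parses ReturnedText immediately, without awaiting that response.
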(event Custom|StartVoiceAssistant
  (params (VoiceResponseAudio :type Sound%20Base%20Object%20Reference))
  (bind _audio (Variables|Default|GetAudio))
  ;[1 1 1] Voice Sounds
  (Audio|Components|Audio|SetSound _audio VoiceResponseAudio)
  (Audio|Components|Audio|Play _audio 0.0))

(event Custom|InvestigationIcon
  (bind _investigatewidget (Variables|Default|GetInvestigateWidget))
  ;[1 1 1] Investigation Mark when sound event occurs
  (Utilities|FlowControl|FlipFlop
    (:A
      (Rendering|SetVisibility _investigatewidget true false))
    (:B
      (Rendering|SetVisibility _investigatewidget false false))))

(event Custom|OnPopulateAudioData_Event
  (params (PopulatedAudioData :type Array%20of%20Floats%20%28single-precision%29))
  (bind _capturablesoundwave (Variables|Default|GetCapturableSoundWave))
  ;[1 1 1] Voice Recognition
  (Class|SpeechRecognizer|ProcessAudioData (Variables|Default|GetSpeechRecognizer) PopulatedAudioData (Math|Conversions|ToFloat(Integer) (Class|ImportedSoundWave|GetSampleRate _capturablesoundwave)) (Class|ImportedSoundWave|GetNumOfChannels _capturablesoundwave) false))

(event Custom|OnStartSpeechRecognition_Event
  (params (bSucceeded :type Boolean))
  ;[1 1 1] Voice Recognition
  (bind _returnvalue (Class|CapturableSoundWave|CreateCapturableSoundWave))
  (bind _output_get (Variables|Default|SetCapturableSoundWave _returnvalue))
  (EventDispatchers|BindEventtoOnPopulateAudioData _output_get (delegate Custom|OnPopulateAudioData_Event))
  (Class|CapturableSoundWave|StartCapture (Variables|Default|GetCapturableSoundWave)))

(event Custom|OpenChat
  ;[1 1 1] Open and Close Chatwindow
  (if (not (Variables|Default|GetChatOpen))
    (UserInterface|Viewport|AddtoViewport (Variables|Default|GetChatWidRef) 0)
    (Variables|Default|SetChatOpen true)))

(event Custom|OpenShopCommand
  (bind _shopref (Variables|Default|GetShopRef))
  ;[1 1 1] Shop Window
  (if (Variables|Default|GethasShop)
    (Utilities|FlowControl|Delay 2.0)
    (UserInterface|Viewport|AddtoViewport _shopref 0)
    (Input|SetInputModeUIOnly (Game|GetPlayerController 0) _shopref "DoNotLock" false)))

(event Custom|QIsPressed
  (bind _chatwindowref (Variables|Default|GetChatWindowRef))
  ;[1 1 1] Voice Recognition
  (if (Variables|Default|GetChatOpen)
    (Default|CreateSpeechBubble _chatwindowref)
    (Development|PrintString "RECORDING STARTED" true true "(R=1.000000,G=0.000000,B=0.075999,A=1.000000)")
    (bind _returnvalue (Class|SpeechRecognizer|CreateSpeechRecognizer))
    (bind _output_get (Variables|Default|SetSpeechRecognizer _returnvalue))
    (Development|PrintString "VOICE RECOGNITION STARTED" true true "(R=0.000000,G=1.000000,B=0.449602,A=1.000000)")
    (EventDispatchers|BindEventtoOnRecognitionFinished _output_get (delegate Custom|OnRecognitionFinished_Event))
    (EventDispatchers|BindEventtoOnRecognitionError _output_get (delegate Custom|OnRecognitionError_Event))
    (EventDispatchers|BindEventtoOnRecognizedTextSegment (Variables|Default|GetSpeechRecognizer) (delegate Custom|OnRecognizedTextSegment_Event))
    (Class|SpeechRecognizer|SetStreamingDefaults (Variables|Default|GetSpeechRecognizer))
    (Class|SpeechRecognizer|SetLanguage (Variables|Default|GetSpeechRecognizer) "En")
    (Class|SpeechRecognizer|StartSpeechRecognition (Variables|Default|GetSpeechRecognizer) (delegate Custom|OnStartSpeechRecognition_Event))
    (else
      (Default|DestroySpeechBubble _chatwindowref)
      (Class|CapturableSoundWave|StopCapture (Variables|Default|GetCapturableSoundWave))
      (Class|SpeechRecognizer|ForceProcessPendingAudioData (Variables|Default|GetSpeechRecognizer)))))

(event Custom|QIsReleased
  ;[1 1 1] Voice Recognition
  (Default|DestroySpeechBubble (Variables|Default|GetChatWindowRef))
  (Class|CapturableSoundWave|StopCapture (Variables|Default|GetCapturableSoundWave))
  (Class|SpeechRecognizer|ForceProcessPendingAudioData (Variables|Default|GetSpeechRecognizer)))

(event Custom|RotateToPlayerCheck
  (bind _interacttextref (Variables|Default|GetInteractTextRef))
  ;[1 1 1] ChatboxControl
  (CallFunction|RotationtoPlayer)
  (if (Variables|Default|GetChatOpen)
    (Utilities|IsValid _interacttextref
      (:Is%20Valid
        (Widget|RemovefromParent _interacttextref)))))

(event Custom|SendText
  (params (InputPrompt :type String))
  (bind _returnvalue (Utilities|String|Append "user:" InputPrompt))
  ;[1 1 1] ConversationMemory | "ShortTerm Memory"
  (Development|PrintString InputPrompt true true "(R=0.000000,G=0.660000,B=1.000000,A=1.000000)" 12.0)
  (Utilities|Array|Add (Variables|Default|GetConversation%20Array) _returnvalue)
  (Variables|Default|SethasSentChat true)
  (CallFunction|EnterVoicePrompt _returnvalue))

(event Custom|RunSpeechReply
  (params (GPTReply :type String))
  ;[1 1 1] VoiceReply
  (Development|PrintString "Creating Voice Reply" true true "(R=1.000000,G=0.938499,B=0.000000,A=1.000000)" 5.0)
  (bind _output_get (Variables|Default|SetGPTReply GPTReply))
  (bind _returnvalue (Class|VaRestSubsystem|ConstructVaRestRequestExt (|VaRestSubsystem) "POST" "json"))
  (Class|VaRestRequestJSON|SetRequestObject _returnvalue (|MakeJson _output_get "eleven_monolingual_v1" (|MakeJson 0.1 0.1)))
  (Class|VaRestRequestJSON|SetHeader _returnvalue "accept" "audio/mpeg")
  (Class|VaRestRequestJSON|SetHeader _returnvalue "xi-api-key" (Variables|Default|GetElevenLabsAPIKey))
  (Class|VaRestRequestJSON|SetHeader _returnvalue "Content-Type" "application/json")
  (Class|VaRestRequestJSON|ProcessURL _returnvalue (Utilities|Array|Get(acopy) (Variables|Default|GetVoiceAPIArray) (Variables|Default|GetVoiceIndex)))
  (EventDispatchers|BindEventtoOnRequestComplete _returnvalue (delegate Custom|VoiceRequestComplete))
  (EventDispatchers|BindEventtoOnRequestFail _returnvalue (delegate Custom|SpeechRequestFailed)))

(event Custom|TargetPlayer
  (bind _returnvalue (Pawn|GetController))
  (bind _playerref (Variables|Default|GetPlayerRef))
  (bind _currentaispokento (Variables|/Game/ThirdPerson/Blueprints/BP_Player.BP_Player_C|GetCurrentAISpokenTo _playerref))
  ;[1 1 1] Target and Untarget Player
  (AI|AIMoveTo _currentaispokento "0, 0, 0" _playerref 1.5e+02 false
    (:then
      (Transformation|SetActorRotation _currentaispokento (Math|Rotator|MakeRotator 0.0 0.0 (+ (.yaw (Transformation|GetActorRotation _playerref)) 1.8e+02)))
      ;[1 1 1] Freeze Movement
      (Variables|/Script/Engine.MovementComponent|SetVelocity (Variables|/Script/Engine.Character|GetCharacterMovement (Variables|/Game/ThirdPerson/Blueprints/BP_Player.BP_Player_C|GetCurrentAISpokenTo (Variables|Default|GetPlayerRef))) "0, 0, 0")
      (Input|SetIgnoreMoveInput _returnvalue false)
      (Input|SetIgnoreLookInput _returnvalue false))))

(event Custom|GPTRequestFailed
  (params (Request :type Va%20Rest%20Request%20JSON%20Object%20Reference))
  ;[1 1 1] GPT Response
  (Development|PrintString "GPT Request FAILED" true true "(R=1.000000,G=0.034090,B=0.000000,A=1.000000)" 1e+01))

(event Custom|UnTargetPlayer
  ;[1 1 1] Target and Untarget Player
  (Pawn|Components|CharacterMovement|SetMovementMode (Variables|Character|GetCharacterMovement) "MOVE_NavWalking" 0))

(event Custom|RotationToPlayer
  ;[1 1 1] Rotation
  (Transformation|SetWorldRotation (Variables|Default|GetInvestigateWidget) (Math|Rotator|FindLookatRotation (Transformation|GetWorldLocation (Variables|Default|GetInvestigateWidget)) (Transformation|GetWorldLocation (Variables|/Script/Engine.PlayerCameraManager|GetTransformComponent (Game|GetPlayerCameraManager 0)))) false false)
  (bind _asbp_player (Utilities|Casting|CastToBP_Player (Game|GetPlayerCharacter 0)))
  (Variables|Default|SetPlayerRef _asbp_player)
  (if (Variables|/Game/ThirdPerson/Blueprints/BP_Player.BP_Player_C|GetisInteracting _asbp_player)
    (CallFunction|TargetPlayer)
    (else
      (CallFunction|UnTargetPlayer))))

(event Custom|GPTRequestComplete
  (params (Request :type Va%20Rest%20Request%20JSON%20Object%20Reference))
  (bind _returnvalue (Class|VaRestRequestJSON|GetResponseObject Request))
  (bind _writtenchatref (Variables|Default|GetWrittenChatRef))
  (bind _chatwindowref (Variables|Default|GetChatWindowRef))
  (bind _returnvalue_2 (Class|VaRestJsonObject|GetObjectArrayField _returnvalue "choices"))
  (bind _scroll_aichat (Variables|/Game/_mystuff/HUD/BP_WrittenChat.BP_WrittenChat_C|GetScroll_AIChat _writtenchatref))
  (bind _scroll_aichat_2 (Variables|/Game/_mystuff/HUD/BP_Chat.BP_Chat_C|GetScroll_AIChat _chatwindowref))
  (bind _output (Utilities|Array|Get(acopy) _returnvalue_2))
  (bind _message (|BreakJson _output))
  (bind _content (|BreakJson _message))
  ;[1 1 1] GPT Response
  (bind _returnvalue_3 (Class|VaRestRequestJSON|GetResponseContentasString Request true))
  (Variables|Default|SetReturnedText _returnvalue_3)
  (if (Utilities|String|Contains (Variables|Default|GetReturnedText) "ERROR")
    (Development|PrintString "OPEN AI NO TOKENS LEFT" true true "(R=1.000000,G=0.019096,B=0.000000,A=1.000000)")
    (else
      (Development|PrintString _content true true "(R=0.000000,G=0.660000,B=1.000000,A=1.000000)" 1e+01)
      (if (not (Variables|Default|GetisMemory))
        (Utilities|FlowControl|Sequence
          (:then_0
            (Utilities|Array|Add (Variables|Default|GetConversation%20Array) (Utilities|String|Append "system:" _content))
            (if (Utilities|String|Contains (Variables|Default|GetReturnedText) "OPEN_SHOP")
              (CallFunction|OpenShopCommand))
            (CallFunction|RunSpeechReply (Utilities|String|Replace (Utilities|String|Replace (Utilities|String|Replace (Utilities|String|Replace _content "system:" " ") "user:" " ") (Utilities|String|Append (Variables|Default|GetNPCName) ":") " ") "<OPEN_SHOP>" " ")))
          (:then_1
            (bind _returnvalue_4 (UserInterface|CreateWidget "/Game/_mystuff/HUD/BP_AIText.BP_AIText_C" (Game|GetPlayerController 0) (Utilities|Text|ToText(String) _content) "(R=0.052370,G=1.000000,B=0.105133,A=1.000000)"))
            (bind _asbp_player (Utilities|Casting|CastToBP_Player (Game|GetPlayerCharacter 0)))
            (if (Variables|/Game/ThirdPerson/Blueprints/BP_Player.BP_Player_C|GetwantsVoice _asbp_player)
              (Widget|Panel|AddChild _scroll_aichat_2 _returnvalue_4)
              (Class|ScrollBox|SetScrollOffset _scroll_aichat_2 (Class|ScrollBox|GetScrollOffsetOfEnd _scroll_aichat_2))
              (else
                (Widget|Panel|AddChild _scroll_aichat _returnvalue_4)
                (Class|ScrollBox|SetScrollOffset _scroll_aichat (Class|ScrollBox|GetScrollOffsetOfEnd _scroll_aichat))))))))))

(event Custom|AddRecentMemory
  (bind _returnedtext (Variables|Default|GetReturnedText))
  (bind _returnvalue (Utilities|String|FindSubstring _returnedtext "INTERACTION_DETAIL"))
  (bind _returnvalue_2 (Utilities|String|FindSubstring _returnedtext "OUTCOME_TYPE"))
  (bind _returnvalue_3 (Utilities|String|FindSubstring _returnedtext "INTERACTION_TYPE"))
  ;[1 1 1] add memory
  (for _array_element (Variables|Default|GetConversation%20Array)
    (bind _output_get (Variables|Default|SetJoinedConversationString (Utilities|String|Append (stale _output_get) _array_element))))
  (Variables|Default|SetisMemory true)
  (bind _output_get_2 (Variables|Default|SetRecentMemoryPrompt (Utilities|String|Append "Analyze the Interaction. 
I need 3 different things from you that determine how your memory will function. These words will be stored into an array for future prompts, so choose carefully what is important from the conversation. 
Give me the Interaction Type in one word. write <INTERACTION_TYPE> before the actual word to initiate a variable. 
write <INTERACTION_TYPE_END> to end the variable. 
 
Give me the Interaction Detail and describe in very simple words what has happened. write <INTERACTION_DETAIL> before the text to initiate a variable. write <INTERACTION_DETAIL_END> to end the variable. 
 
Give me the Interaction Outcome. Determine what the outcome of this Interaction was. This can be a feeling towards the other user. Write <OUTCOME_TYPE> in front of your simple explanaition to initiate a variable. write <OUTCOME_TYPE_END> to end the variable." (Variables|Default|GetJoinedConversationString))))
  (Variables|Default|SetInputPrompt _output_get_2)
  (CallFunction|SendJSON)
  (Variables|Default|SetMemoryLog (Utilities|Array|MakeArray (Utilities|Struct|MakeS_MemoryEntry (Utilities|String|GetSubstring _returnedtext _returnvalue_3 (- (Utilities|String|FindSubstring _returnedtext "INTERACTION_TYPE_END") _returnvalue_3)) (Utilities|String|GetSubstring _returnedtext _returnvalue (- (Utilities|String|FindSubstring _returnedtext "INTERACTION_DETAIL_END") _returnvalue)) (Utilities|String|GetSubstring _returnedtext _returnvalue_2 (- (Utilities|String|FindSubstring _returnedtext "OUTCOME_TYPE_END") _returnvalue_2)) "0001.01.01-00.00.00"))))

(event Custom|SetMainInputPrompt
  (bind _memorylog (Variables|Default|GetMemoryLog))
  (bind _output (Utilities|Array|Get(acopy) _memorylog))
  ;[1 1 1] MemoryStream | "LongTerm Memory" + Perception
  (Variables|Default|SetMainInputPrompt (Utilities|String|Append (Utilities|String|Append (Variables|Default|GetContextPrompt) "Setting: " (Variables|Default|GetSettingPrompt) "The following is your Job: " (Variables|Default|GetJobPrompt) "The following is the current Atmosphere: " (Variables|Default|GetAtmospherePrompt) "This is how you feel: " (Variables|Default|GetCurrentFeelingPrompt) "This is your Name: " (Variables|Default|GetNPCName) "This is your current Location: " (Variables|Default|GetNPCContextLocation) "This is the current Time: " (Variables|Default|GetTimePrompt) "Here are some additional Informations: " (Variables|Default|GetadditionalInfo) (Variables|Default|GetShopPrompt)) (Utilities|String|Append "The following text is your current memory: " (.interactiontype _output) (.interactiondetail _output) (.outcome _output)))))

(event Custom|SendJSON
  ;[1 1 1] GPT Response
  (bind _returnvalue (Class|VaRestSubsystem|ConstructVaRestRequestExt (|VaRestSubsystem) "POST" "json"))
  (Class|VaRestRequestJSON|SetRequestObject _returnvalue (|MakeJson (Variables|Default|GetModel) (Utilities|Array|MakeArray (|MakeJson "system" (Variables|Default|GetMainInputPrompt)) 0 (|MakeJson "user" (Utilities|String|Append (Variables|Default|GetPlayerGivenName) ":" (Variables|Default|GetInputPrompt)))) 3e+01))
  (Class|VaRestRequestJSON|SetHeader _returnvalue "Authorization" (Utilities|String|Append "Bearer " (Variables|Default|GetOpenAIAPIKey)))
  (Class|VaRestRequestJSON|SetHeader _returnvalue "Content-Type" "application/json")
  (Class|VaRestRequestJSON|ProcessURL _returnvalue "https://api.openai.com/v1/chat/completions")
  (EventDispatchers|BindEventtoOnRequestComplete _returnvalue (delegate Custom|GPTRequestComplete))
  (EventDispatchers|BindEventtoOnRequestFail _returnvalue (delegate Custom|GPTRequestFailed)))

(event Custom|UpdateSpeech
  (bind _returnvalue (Game|GetPlayerController 0))
  ;[1 1 1] InitWidgets
  (CallFunction|SetMainInputPrompt)
  (Utilities|FlowControl|Sequence
    (:then_0
      ;[1 1 1] get Time of Day
      (bind _returnvalue_2 (Actor|GetActorOfClass "/Game/_mystuff/Managers/BP_DayNightCycle.BP_DayNightCycle_C"))
      (Variables|Default|SetTimeObject _returnvalue_2))
    (:then_1
      (bind _returnvalue_3 (UserInterface|CreateWidget "/Game/_mystuff/HUD/BP_WrittenChat.BP_WrittenChat_C" (Game|GetPlayerController 0)))
      (bind _output_get (Variables|Default|SetWrittenChatRef _returnvalue_3))
      (bind _returnvalue_4 (UserInterface|CreateWidget "/Game/_mystuff/HUD/BP_Chat.BP_Chat_C" (Game|GetPlayerController 0)))
      (bind _output_get_2 (Variables|Default|SetChatWindowRef _returnvalue_4))
      (if (Variables|Default|GetVoiceChat)
        (Variables|Default|SetChatWidRef _output_get_2)
        (else
          (Variables|Default|SetChatWidRef _output_get)))
      (bind _returnvalue_5 (UserInterface|CreateWidget "/Game/_mystuff/HUD/BP_InteractText.BP_InteractText_C" _returnvalue))
      (Variables|Default|SetInteractTextRef _returnvalue_5)
      (bind _returnvalue_6 (UserInterface|CreateWidget "/Game/_mystuff/HUD/BP_SpeechText.BP_SpeechText_C" _returnvalue))
      (Variables|Default|SetSpeechTextRef _returnvalue_6)
      (bind _returnvalue_7 (UserInterface|CreateWidget "/Game/_mystuff/HUD/BP_Shop.BP_Shop_C" _returnvalue))
      (Variables|Default|SetShopRef _returnvalue_7))))

(event Custom|OnRecognitionFinished_Event
  ;[1 1 1] Voice Recognition
  (if (not (Class|CapturableSoundWave|IsCapturing (Variables|Default|GetCapturableSoundWave)))
    (Class|SpeechRecognizer|StopSpeechRecognition (Variables|Default|GetSpeechRecognizer))
    (Variables|Default|SetSpeechRecognizer 0)
    (Development|PrintString "VOICE RECOGNITION STOPPED" true true "(R=1.000000,G=0.921913,B=0.178997,A=1.000000)" 3.0)))

(event Custom|SpeechRequestFailed
  (params (Request :type Va%20Rest%20Request%20JSON%20Object%20Reference))
  ;[1 1 1] VoiceReply
  (Development|PrintString "Speech Request Failed"))

(event Custom|EnterVoicePrompt
  (params (InputPrompt :type String))
  ;[1 1 1] GPT Response
  (if (Variables|Default|GethasShop)
    (Variables|Default|SetShopPrompt "\"send the following text when the player wants to see your wares: <OPEN_SHOP>\""))
  (Development|PrintString "Prompt ChatGPT" true true "(R=0.000000,G=0.660000,B=1.000000,A=1.000000)" 5.0)
  (Variables|Default|SetInputPrompt (Utilities|String|JoinStringArray (Variables|Default|GetConversation%20Array) " "))
  (bind _returnvalue (Class|VaRestSubsystem|ConstructVaRestRequestExt (|VaRestSubsystem) "POST" "json"))
  (Class|VaRestRequestJSON|SetRequestObject _returnvalue (|MakeJson (Variables|Default|GetModel) (Utilities|Array|MakeArray (|MakeJson "system" (Variables|Default|GetMainInputPrompt)) 0 (|MakeJson "user" (Utilities|String|Append (Variables|Default|GetPlayerGivenName) ":" (Variables|Default|GetInputPrompt)))) 3e+01))
  (Class|VaRestRequestJSON|SetHeader _returnvalue "Authorization" (Utilities|String|Append "Bearer " (Variables|Default|GetOpenAIAPIKey)))
  (Class|VaRestRequestJSON|SetHeader _returnvalue "Content-Type" "application/json")
  (Class|VaRestRequestJSON|ProcessURL _returnvalue "https://api.openai.com/v1/chat/completions")
  (EventDispatchers|BindEventtoOnRequestComplete _returnvalue (delegate Custom|GPTRequestComplete))
  (EventDispatchers|BindEventtoOnRequestFail _returnvalue (delegate Custom|GPTRequestFailed)))

(event Custom|VoiceRequestComplete
  (params (Request :type Va%20Rest%20Request%20JSON%20Object%20Reference))
  ;[1 1 1] VoiceReply
  (bind _returnvalue (Class|VaRestRequestJSON|GetResponseContentasString Request true))
  (if (Utilities|String|Contains _returnvalue "exceed")
    (Development|PrintString "RAN OUT OF ELEVENLABS TOKENS" true true "(R=1.000000,G=0.020229,B=0.000000,A=1.000000)" 1e+01)
    (else
      (bind _returnvalue_2 (Class|RuntimeAudioImporterLibrary|CreateRuntimeAudioImporter))
      (bind _output_get (Variables|Default|SetImporter _returnvalue_2))
      (EventDispatchers|BindEventtoOnResult _output_get (delegate Custom|OnResult))
      (Class|RuntimeAudioImporterLibrary|ImportAudiofromBuffer _output_get (Class|VaRestRequestJSON|GetResponseContent Request) "Mp3"))))

(event Custom|OnResult
  (params (Importer :type Runtime%20Audio%20Importer%20Library%20Object%20Reference) (ImportedSoundWave :type Imported%20Sound%20Wave%20Object%20Reference) (Status :type ERuntimeImportStatus%20Enum :default "SuccessfulImport"))
  ;[1 1 1] VoiceReply
  (Development|PrintString "PLAYING VOICE REPLY" true true "(R=0.000000,G=1.000000,B=0.054741,A=1.000000)" 5.0)
  (CallFunction|StartVoiceAssistant ImportedSoundWave))

(event Custom|CloseChat
  (bind _playerref (Variables|Default|GetPlayerRef))
  (bind _returnvalue (Pawn|GetController _playerref))
  ;[1 1 1] Open and Close Chatwindow
  (Default|UnsetInputMode (Variables|Default|GetWrittenChatRef))
  (Widget|RemovefromParent (Variables|Default|GetChatWidRef))
  (Variables|Default|SetChatOpen false)
  (if (Variables|Default|GethasSentChat)
    (Variables|Default|SethasSentChat false)
    (CallFunction|AddRecentMemory))
  (Input|SetIgnoreMoveInput _returnvalue false)
  (Input|SetIgnoreLookInput _returnvalue false))

(event Custom|OnRecognitionError_Event
  (params (ShortErrorMessage :type String) (LongErrorMessage :type String))
  ;[1 1 1] Voice Recognition
  (Development|PrintString LongErrorMessage true true "(R=1.000000,G=0.000000,B=0.000000,A=1.000000)" 15.0))

(event Custom|OnRecognizedTextSegment_Event
  (params (RecognizedWords :type String))
  (bind _returnvalue (Utilities|String|Append "user:" RecognizedWords))
  ;[1 1 1] Voice Recognition
  (Development|PrintString RecognizedWords true true "(R=0.000000,G=0.660000,B=1.000000,A=1.000000)" 12.0)
  (Utilities|FlowControl|Sequence
    (:then_0
      (bind _returnvalue_2 (UserInterface|CreateWidget "/Game/_mystuff/HUD/BP_AIText.BP_AIText_C" (Game|GetPlayerController 0) (Utilities|Text|ToText(String) _returnvalue) "(R=1.000000,G=1.000000,B=1.000000,A=1.000000)"))
      (Widget|Panel|AddChild (Variables|/Game/_mystuff/HUD/BP_Chat.BP_Chat_C|GetScroll_AIChat (Variables|Default|GetChatWindowRef)) _returnvalue_2))
    (:then_1
      (Utilities|Array|Add (Variables|Default|GetConversation%20Array) _returnvalue)
      (CallFunction|EnterVoicePrompt _returnvalue))))

(event EventBeginPlay
  (bind _returnvalue (Game|GetPlayerController 0))
  ;[1 1 1] InitWidgets
  (CallFunction|SetMainInputPrompt)
  (Utilities|FlowControl|Sequence
    (:then_0
      ;[1 1 1] get Time of Day
      (bind _returnvalue_2 (Actor|GetActorOfClass "/Game/_mystuff/Managers/BP_DayNightCycle.BP_DayNightCycle_C"))
      (Variables|Default|SetTimeObject _returnvalue_2))
    (:then_1
      (bind _returnvalue_3 (UserInterface|CreateWidget "/Game/_mystuff/HUD/BP_WrittenChat.BP_WrittenChat_C" (Game|GetPlayerController 0)))
      (bind _output_get (Variables|Default|SetWrittenChatRef _returnvalue_3))
      (bind _returnvalue_4 (UserInterface|CreateWidget "/Game/_mystuff/HUD/BP_Chat.BP_Chat_C" (Game|GetPlayerController 0)))
      (bind _output_get_2 (Variables|Default|SetChatWindowRef _returnvalue_4))
      (if (Variables|Default|GetVoiceChat)
        (Variables|Default|SetChatWidRef _output_get_2)
        (else
          (Variables|Default|SetChatWidRef _output_get)))
      (bind _returnvalue_5 (UserInterface|CreateWidget "/Game/_mystuff/HUD/BP_InteractText.BP_InteractText_C" _returnvalue))
      (Variables|Default|SetInteractTextRef _returnvalue_5)
      (bind _returnvalue_6 (UserInterface|CreateWidget "/Game/_mystuff/HUD/BP_SpeechText.BP_SpeechText_C" _returnvalue))
      (Variables|Default|SetSpeechTextRef _returnvalue_6)
      (bind _returnvalue_7 (UserInterface|CreateWidget "/Game/_mystuff/HUD/BP_Shop.BP_Shop_C" _returnvalue))
      (Variables|Default|SetShopRef _returnvalue_7))))

(event Collision|EventActorEndOverlap
  (params (OtherActor :type Actor%20Object%20Reference))
  (bind _interacttextref (Variables|Default|GetInteractTextRef))
  ;[1 1 1] ChatboxControl
  (Utilities|Casting|CastToBP_Player OtherActor)
  (Variables|Default|SetinRange false)
  (CallFunction|CloseChat)
  (Utilities|IsValid _interacttextref
    (:Is%20Valid
      (Widget|RemovefromParent _interacttextref))))

(event Collision|EventActorBeginOverlap
  (params (OtherActor :type Actor%20Object%20Reference))
  ;[1 1 1] ChatboxControl
  (Utilities|Casting|CastToBP_Player OtherActor)
  (Variables|Default|SetinRange true)
  (UserInterface|Viewport|AddtoViewport (Variables|Default|GetInteractTextRef) 0))

(event EventTick
  (params (DeltaSeconds :type Float%20%28single-precision%29))
  ;[1 1 1] Event Tick
  (CallFunction|RotatetoPlayerCheck)
  (Variables|Default|SetTimePrompt (Utilities|String|ToString(Float) (Variables|/Game/_mystuff/Managers/BP_DayNightCycle.BP_DayNightCycle_C|GetTimeOfDay (Variables|Default|GetTimeObject)))))

(fn ConstructionScript)

(fn AddMemory
  (params (InteractionType :type String) (InteractionDetail :type String) (Outcome :type String) (Timestamp :type Date%20Time%20Structure))
  (bind _output_get (LocalVariables|SetNewMemoryEntry (Utilities|Struct|MakeS_MemoryEntry InteractionType InteractionDetail Outcome Timestamp)))
  (Utilities|Array|Add (Variables|Default|GetMemoryLog) _output_get))