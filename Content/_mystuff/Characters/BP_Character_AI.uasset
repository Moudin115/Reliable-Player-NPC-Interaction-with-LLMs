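; BP_Character_AI is an AI character with a world-space investigate icon and an attack function.
; Tick rotates the InvestigateWidget to face the player camera each frame.
; The InvestigationIcon event uses a FlipFlop to show and hide that widget on alternate calls.
; Attack calls PlayAnimMontage with no montage specified in the graph and returns a constant zero.
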(event Custom|InvestigationIcon
  (bind _investigatewidget (Variables|Default|GetInvestigateWidget))
  (Utilities|FlowControl|FlipFlop
    (:A
      (Rendering|SetVisibility _investigatewidget true false))
    (:B
      (Rendering|SetVisibility _investigatewidget false false))))

(event EventTick
  (params (DeltaSeconds :type Float%20%28single-precision%29))
  (Transformation|SetWorldRotation (Variables|Default|GetInvestigateWidget) (Math|Rotator|FindLookatRotation (Transformation|GetWorldLocation (Variables|Default|GetInvestigateWidget)) (Transformation|GetWorldLocation (Variables|/Script/Engine.PlayerCameraManager|GetTransformComponent (Game|GetPlayerCameraManager 0)))) false false))

(fn ConstructionScript)

(fn Attack
  (Animation|PlayAnimMontage 0 1.0 "None")
  (return 0.0))