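; Talking world object that speaks an AI-generated, in-character line when the player overlaps it and destroys itself when the player leaves.
; BeginPlay assembles a persona prompt, which VaRest sends to Gemini (hardcoded API key in URL) or GPT-3.5, retrying empty Gemini replies.
; The cleaned reply goes to ElevenLabs, and Runtime Audio Importer converts the returned MP3 for playback.
; Tick billboards the plane toward the player camera's yaw.
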(event Custom|StartVoice
  (params (VoiceResponseAudio :type Sound%20Base%20Object%20Reference))
  (bind _audio (Variables|Default|GetAudio))
  (Audio|Components|Audio|SetSound _audio VoiceResponseAudio)
  (Audio|Components|Audio|Play _audio 0.0))

(event Custom|SetPlayer
  ;[1 1 1] set player
  (bind _returnvalue (Actor|GetActorOfClass "/Game/_mystuff/Characters/Player/BP_Player.BP_Player_C"))
  (Utilities|IsValid _returnvalue
    (:Is%20Valid
      (Variables|Default|SetPlayerRef _returnvalue))))

(event Custom|GeminiEventComplete
  (params (Request :type Va%20Rest%20Request%20JSON%20Object%20Reference))
  ;[1 1 1] Gemini JSON Request
  (bind _returnvalue (Class|VaRestRequestJSON|GetResponseContentasString Request true))
  (Variables|Default|SetReturnedText _returnvalue)
  (if (Utilities|String|Contains (Variables|Default|GetReturnedText) "ERROR")
    (Development|PrintString "OPEN AI NO TOKENS LEFT" true true "(R=1.000000,G=0.019096,B=0.000000,A=1.000000)")
    (else
      (CallFunction|GeminiJSONOutput))))

(event Custom|GPTRequestFailed
  (params (Request :type Va%20Rest%20Request%20JSON%20Object%20Reference))
  ;[1 1 1] GPT Code
  (Development|PrintString "GPT Request FAILED" true true "(R=1.000000,G=0.034090,B=0.000000,A=1.000000)" 1e+01))

(event Custom|GPTOutput
  ;[1 1 1] GPT Code
  (Development|PrintString (|BreakJson (|BreakJson (Utilities|Array|Get(acopy) (Class|VaRestJsonObject|GetObjectArrayField (Class|VaRestRequestJSON|GetResponseObject (stale Custom|GPTRequestComplete Request)) "choices")))) true true "(R=0.000000,G=0.660000,B=1.000000,A=1.000000)" 1e+01)
  (Utilities|Array|Add (Variables|Default|GetConversationArray) (Utilities|String|Append "system:" (|BreakJson (|BreakJson (Utilities|Array|Get(acopy) (Class|VaRestJsonObject|GetObjectArrayField (Class|VaRestRequestJSON|GetResponseObject (stale Custom|GPTRequestComplete Request)) "choices"))))))
  (CallFunction|RunSpeechReply (Utilities|String|Replace (Utilities|String|Replace (Utilities|String|Replace (|BreakJson (|BreakJson (Utilities|Array|Get(acopy) (Class|VaRestJsonObject|GetObjectArrayField (Class|VaRestRequestJSON|GetResponseObject (stale Custom|GPTRequestComplete Request)) "choices")))) "system:" " ") "user:" " ") (Utilities|String|Append (Variables|Default|GetNPCName) ":") " ")))

(event Custom|GPTRequestComplete
  (params (Request :type Va%20Rest%20Request%20JSON%20Object%20Reference))
  ;[1 1 1] GPT Code
  (bind _returnvalue (Class|VaRestRequestJSON|GetResponseContentasString Request true))
  (Variables|Default|SetReturnedText _returnvalue)
  (if (Utilities|String|Contains (Variables|Default|GetReturnedText) "ERROR")
    (Development|PrintString "OPEN AI NO TOKENS LEFT" true true "(R=1.000000,G=0.019096,B=0.000000,A=1.000000)")
    (else
      (CallFunction|GPTOutput))))

(event Custom|RunSpeechReply
  (params (GPTReply :type String))
  ;[1 1 1] VoiceReply
  (Development|PrintString "Creating Voice Reply" true true "(R=1.000000,G=0.938499,B=0.000000,A=1.000000)" 5.0)
  (bind _output_get (Variables|Default|SetGPTReply GPTReply))
  (bind _returnvalue (Class|VaRestSubsystem|ConstructVaRestRequestExt (|VaRestSubsystem) "POST" "json"))
  (Class|VaRestRequestJSON|SetRequestObject _returnvalue (|MakeJson _output_get "eleven_monolingual_v1" (|MakeJson 0.1 0.1)))
  (Class|VaRestRequestJSON|SetHeader _returnvalue "accept" "audio/mpeg")
  (Class|VaRestRequestJSON|SetHeader _returnvalue "xi-api-key" (Variables|Default|GetElevenLabsAPIKey))
  (Class|VaRestRequestJSON|SetHeader _returnvalue "Content-Type" "application/json")
  (Class|VaRestRequestJSON|ProcessURL _returnvalue (Utilities|Array|Get(acopy) (Variables|Default|GetVoiceAPIArray) (Variables|Default|GetVoiceIndex)))
  (EventDispatchers|BindEventtoOnRequestComplete _returnvalue (delegate Custom|VoiceRequestComplete))
  (EventDispatchers|BindEventtoOnRequestFail _returnvalue (delegate Custom|SpeechRequestFailed)))

(event Custom|GeminiFailed
  (params (Request :type Va%20Rest%20Request%20JSON%20Object%20Reference))
  (Development|PrintString "Gemini Request FAILED" true true "(R=1.000000,G=0.034090,B=0.000000,A=1.000000)" 1e+01))

(event Custom|SetMainInputPrompt
  ;[1 1 1] Main Input Prompt
  (Variables|Default|SetMainInputPrompt (Utilities|String|Append (Variables|Default|GetContextPrompt) "Setting: " (Variables|Default|GetSettingPrompt) "The following is your Job: " (Variables|Default|GetJobPrompt) "The following is the current Atmosphere: " (Variables|Default|GetAtmospherePrompt) "This is how you feel: " (Variables|Default|GetCurrentFeelingPrompt) "This is your Name: " (Variables|Default|GetNPCName) "This is your current Location: " (Variables|Default|GetNPCContextLocation) "This is the current Time: " (Variables|Default|GetTimePrompt) "Here are some additional Informations: " (Variables|Default|GetadditionalInfo) "Talk about something on your mind" "You do not need any additional information. Just talk as a Character!")))

(event Custom|ActivateVoice
  (if (Variables|Default|GetisGemini)
    (CallFunction|GeminiRequest)
    (Development|PrintString "LLM Object ACTIVATED")
    (else
      (CallFunction|GPTRequest))))

(event Custom|GeminiJSONOutput
  ;[1 1 1] Gemini Response
  (if (Utilities|Array|IsEmpty (|BreakJson (Utilities|Array|Get(acopy) (Class|VaRestJsonObject|GetObjectArrayField (|BreakJson (Utilities|Array|Get(acopy) (Class|VaRestJsonObject|GetObjectArrayField (Class|VaRestRequestJSON|GetResponseObject (stale Custom|GeminiEventComplete Request)) "candidates"))) "Parts"))))
    (CallFunction|ActivateVoice)
    (else
      (Development|PrintString (|BreakJson (Utilities|Array|Get(acopy) (Class|VaRestJsonObject|GetObjectArrayField (|BreakJson (Utilities|Array|Get(acopy) (Class|VaRestJsonObject|GetObjectArrayField (Class|VaRestRequestJSON|GetResponseObject (stale Custom|GeminiEventComplete Request)) "candidates"))) "Parts"))) true true "(R=0.000000,G=0.660000,B=1.000000,A=1.000000)" 1e+01)
      (CallFunction|RunSpeechReply (Utilities|String|Replace (Utilities|String|Replace (Utilities|String|Replace (Utilities|String|Replace (|BreakJson (Utilities|Array|Get(acopy) (Class|VaRestJsonObject|GetObjectArrayField (|BreakJson (Utilities|Array|Get(acopy) (Class|VaRestJsonObject|GetObjectArrayField (Class|VaRestRequestJSON|GetResponseObject (stale Custom|GeminiEventComplete Request)) "candidates"))) "Parts"))) "system:" " ") "user:" " ") (Utilities|String|Append (Variables|Default|GetNPCName) ":") " ") "<OPEN_SHOP>" " ")))))

(event Custom|SpeechRequestFailed
  (params (Request :type Va%20Rest%20Request%20JSON%20Object%20Reference))
  ;[1 1 1] VoiceReply
  (Development|PrintString "Speech Request Failed"))

(event Custom|VoiceRequestComplete
  (params (Request :type Va%20Rest%20Request%20JSON%20Object%20Reference))
  ;[1 1 1] VoiceReply
  (bind _returnvalue (Class|VaRestRequestJSON|GetResponseContentasString Request true))
  (if (Utilities|String|Contains _returnvalue "exceed")
    (Development|PrintString "RAN OUT OF ELEVENLABS TOKENS" true true "(R=1.000000,G=0.020229,B=0.000000,A=1.000000)" 1e+01)
    (else
      (bind _returnvalue_2 (Class|RuntimeAudioImporterLibrary|CreateRuntimeAudioImporter))
      (bind _output_get (Variables|Default|SetImporter _returnvalue_2))
      (EventDispatchers|BindEventtoOnResult _output_get (delegate Custom|OnResult))
      (Class|RuntimeAudioImporterLibrary|ImportAudiofromBuffer _output_get (Class|VaRestRequestJSON|GetResponseContent Request) "Mp3"))))

(event Custom|OnResult
  (params (Importer :type Runtime%20Audio%20Importer%20Library%20Object%20Reference) (ImportedSoundWave :type Imported%20Sound%20Wave%20Object%20Reference) (Status :type ERuntimeImportStatus%20Enum :default "SuccessfulImport"))
  ;[1 1 1] VoiceReply
  (Development|PrintString "PLAYING VOICE REPLY" true true "(R=0.000000,G=1.000000,B=0.054741,A=1.000000)" 5.0)
  (CallFunction|StartVoice ImportedSoundWave))

(event Custom|GPTRequest
  ;[1 1 1] GPT Code
  (bind _returnvalue (Class|VaRestSubsystem|ConstructVaRestRequestExt (|VaRestSubsystem) "POST" "json"))
  (Class|VaRestRequestJSON|SetRequestObject _returnvalue (|MakeJson "gpt-3.5-turbo" (Utilities|Array|MakeArray (|MakeJson "system" (Variables|Default|GetMainInputPrompt)) 0 (|MakeJson "user" (Utilities|String|Append (Variables|Default|GetPlayerGivenName) ":" (Variables|Default|GetMainInputPrompt)))) 3e+01))
  (Class|VaRestRequestJSON|SetHeader _returnvalue "Authorization" (Utilities|String|Append "Bearer " (Variables|Default|GetOpenAIAPIKey)))
  (Class|VaRestRequestJSON|SetHeader _returnvalue "Content-Type" "application/json")
  (Class|VaRestRequestJSON|ProcessURL _returnvalue "https://api.openai.com/v1/chat/completions")
  (EventDispatchers|BindEventtoOnRequestComplete _returnvalue (delegate Custom|GPTRequestComplete))
  (EventDispatchers|BindEventtoOnRequestFail _returnvalue (delegate Custom|GPTRequestFailed)))

(event Custom|GeminiRequest
  ;[1 1 1] Gemini JSON Request
  (bind _returnvalue (Class|VaRestSubsystem|ConstructVaRestRequestExt (|VaRestSubsystem) "POST" "json"))
  (Class|VaRestRequestJSON|SetRequestObject _returnvalue (|MakeJson (|MakeJson (|MakeJson (Utilities|String|Append (Variables|Default|GetMainInputPrompt) (Utilities|String|Append (Variables|Default|GetPlayerGivenName) ":" (Variables|Default|GetMainInputPrompt)))))))
  (Class|VaRestRequestJSON|SetHeader _returnvalue "Content-Type" "application/json")
  (Class|VaRestRequestJSON|ProcessURL _returnvalue "https://generativelanguage.googleapis.com/v1/models/gemini-1.5-flash:generateContent?key=AIzaSyCkpe1l902YliNB1fhPupdrZrsgGRlc9ME")
  (EventDispatchers|BindEventtoOnRequestComplete _returnvalue (delegate Custom|GeminiEventComplete))
  (EventDispatchers|BindEventtoOnRequestFail _returnvalue (delegate Custom|GeminiFailed)))

(event EventBeginPlay
  ;[1 1 1] setup and destroy
  (CallFunction|SetPlayer)
  (CallFunction|SetMainInputPrompt))

(event Collision|EventActorEndOverlap
  (params (OtherActor :type Actor%20Object%20Reference))
  ;[1 1 1] setup and destroy
  (Utilities|Casting|CastToBP_Player OtherActor)
  (Actor|DestroyActor))

(event Collision|EventActorBeginOverlap
  (params (OtherActor :type Actor%20Object%20Reference))
  ;[1 1 1] setup and destroy
  (Utilities|Casting|CastToBP_Player OtherActor)
  (CallFunction|ActivateVoice))

(event EventTick
  (params (DeltaSeconds :type Float%20%28single-precision%29))
  ;[1 1 1] Billboard
  (Transformation|SetWorldRotation (Variables|Default|GetPlane) (Math|Rotator|MakeRotator 9e+01 0.0 (+ (.yaw (Transformation|GetWorldRotation (Variables|/Game/_mystuff/Characters/Player/BP_Player.BP_Player_C|GetFollowCamera (Variables|Default|GetPlayerRef)))) 9e+01)) false false))

(fn ConstructionScript)

(fn StartVoiceAssistant
  (params (VoiceResponseAudio :type Sound%20Base%20Object%20Reference)))