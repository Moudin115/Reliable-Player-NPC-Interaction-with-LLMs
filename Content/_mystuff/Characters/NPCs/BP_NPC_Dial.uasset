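; BP_NPC_Dial is an NPC dialogue Blueprint that shows its Dialogue lines one at a time in a chat widget.
; Each Talk call advances TalkIndex, creates a BP_Chat widget if none is valid, sets its text box and plays a click sound.
; Once the lines run out, Talk removes the widget, clears the reference and resets the index so the conversation can replay.
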(event EventTalk
  (Math|Integer|IncrementInt (Variables|Default|GettalkIndex)
    (:%20%20
      (if (< (Variables|Default|GettalkIndex) (Utilities|Array|Length (Variables|Default|Getdialogue)))
        (Variables|Default|GetUI
          (:then
            _)
          (:else
            (bind _returnvalue (UserInterface|CreateWidget "/Game/_mystuff/HUD/BP_Chat.BP_Chat_C" (Game|GetPlayerController 0)))
            (bind _output_get (Variables|Default|SetUI _returnvalue))
            (UserInterface|Viewport|AddtoViewport _output_get 0)))
        (Rendering|Components|TextRender|SetText (Variables|/Game/_mystuff/HUD/BP_Chat.BP_Chat_C|GetDialogueTextBox (Variables|Default|GetUI)) (Utilities|Text|ToText(String) (Utilities|Array|Get(acopy) (Variables|Default|Getdialogue) (Variables|Default|GettalkIndex))))
        (Audio|PlaySound2D "/Engine/VREditor/Sounds/UI/Click_on_Button.Click_on_Button" 1.0 1.0 0.0 0 0)
        (else
          (Widget|RemovefromParent (Variables|Default|GetUI))
          (Variables|Default|SettalkIndex -1)
          (Variables|Default|SetUI 0))))))

(fn ConstructionScript)