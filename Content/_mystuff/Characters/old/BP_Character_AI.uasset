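; AI character Blueprint that approaches and faces the player during interaction and plays voice responses passed to it.
; Tick billboards the investigate widget to the camera and polls the player's IsInteracting flag to call TargetPlayer or UnTargetPlayer.
; TargetPlayer issues AIMoveTo and sets yaw opposite the player's, while UnTargetPlayer only sets NavWalking movement.
; Events play supplied voice audio and flip-flop the investigation icon; Attack calls PlayAnimMontage without a specified montage.
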(event Custom|StartVoiceAssistant
  (params (VoiceResponseAudio :type Sound%20Base%20Object%20Reference))
  (bind _audio (Variables|Default|GetAudio))
  ;[1 1 1] Voice Sound
  (Audio|Components|Audio|SetSound _audio VoiceResponseAudio)
  (Audio|Components|Audio|Play _audio 0.0))

(event Custom|InvestigationIcon
  (bind _investigatewidget (Variables|Default|GetInvestigateWidget))
  ;[1 1 1] Investigation Mark when sound event occurs
  (Utilities|FlowControl|FlipFlop
    (:A
      (Rendering|SetVisibility _investigatewidget true false))
    (:B
      (Rendering|SetVisibility _investigatewidget false false))))

(event Custom|TargetPlayer
  (bind _playerref (Variables|Default|GetPlayerRef))
  ;[1 1 1] Follow Player
  (AI|AIMoveTo self "0, 0, 0" _playerref 1.5e+02 false
    (:then
      (Transformation|SetActorRotation (Math|Rotator|MakeRotator 0.0 0.0 (+ (.yaw (Transformation|GetActorRotation _playerref)) 1.8e+02))))))

(event Custom|UnTargetPlayer
  ;[1 1 1] Unfollow Player
  (Pawn|Components|CharacterMovement|SetMovementMode (Variables|Character|GetCharacterMovement) "MOVE_NavWalking" 0))

(event EventTick
  (params (DeltaSeconds :type Float%20%28single-precision%29))
  ;[1 1 1] Event Tick
  (Transformation|SetWorldRotation (Variables|Default|GetInvestigateWidget) (Math|Rotator|FindLookatRotation (Transformation|GetWorldLocation (Variables|Default|GetInvestigateWidget)) (Transformation|GetWorldLocation (Variables|/Script/Engine.PlayerCameraManager|GetTransformComponent (Game|GetPlayerCameraManager 0)))) false false)
  (bind _asbp_player (Utilities|Casting|CastToBP_Player (Game|GetPlayerCharacter 0)))
  (Variables|Default|SetPlayerRef _asbp_player)
  (if (Variables|/Game/_mystuff/Characters/Player/BP_Player.BP_Player_C|GetisInteracting _asbp_player)
    (CallFunction|TargetPlayer)
    (else
      (CallFunction|UnTargetPlayer))))

(fn ConstructionScript)

(fn Attack
  (bind _returnvalue (Animation|PlayAnimMontage 0 1.0 "None"))
  (return _returnvalue))