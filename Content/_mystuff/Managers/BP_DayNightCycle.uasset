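; Day-night cycle manager that advances TimeOfDay every tick, wrapping it at the end of the day.
; Each update rotates the referenced sun and moon lights on opposite pitches in proportion to DayLength.
; It also builds a zero-padded HH:MM clock string, offset to start at 08:00 and based on a fixed 600-unit day.
; CheckForMoon toggles light visibility by time window but is never called.
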(event Custom|UpdateTimeOfDay
  (bind _output_get (Variables|Default|SetTimeOfDay (Math|Float|%(Float) (+ (Variables|Default|GetTimeOfDay) (stale EventTick DeltaSeconds)) (Variables|Default|GetDayLength))))
  (if (> _output_get 6e+02)
    (Variables|Default|SetTimeOfDay 0.0))
  (CallFunction|UpdateSunandMoon)
  (Variables|Default|SetcurrentClockTime (Utilities|String|Append (Utilities|String|SelectString (Utilities|String|ToString(Integer) (Class|KismetMathLibrary|ToInt64(Float) (- (+ (/ (Variables|Default|GetTimeOfDay) 25.0) 8.0) 24.0))) (Utilities|String|SelectString (Utilities|String|Append "0" (Utilities|String|ToString(Integer) (Class|KismetMathLibrary|ToInt64(Float) (+ (/ (Variables|Default|GetTimeOfDay) 25.0) 8.0)))) (Utilities|String|ToString(Integer) (Class|KismetMathLibrary|ToInt64(Float) (+ (/ (Variables|Default|GetTimeOfDay) 25.0) 8.0))) (< (+ (/ (Variables|Default|GetTimeOfDay) 25.0) 8.0) 1e+01)) (>= (+ (/ (Variables|Default|GetTimeOfDay) 25.0) 8.0) 24.0)) ":" (Utilities|String|SelectString (Utilities|String|Append "0" (Utilities|String|ToString(Integer) (Class|KismetMathLibrary|ToInt64(Float) (* (Math|Float|Fraction (/ (Variables|Default|GetTimeOfDay) 25.0)) 6e+01)))) (Utilities|String|ToString(Integer) (Class|KismetMathLibrary|ToInt64(Float) (* (Math|Float|Fraction (/ (Variables|Default|GetTimeOfDay) 25.0)) 6e+01))) (< (* (Math|Float|Fraction (/ (Variables|Default|GetTimeOfDay) 25.0)) 6e+01) 1e+01)))))

(event Custom|UpdateSunandMoon
  (bind _timeofday (Variables|Default|GetTimeOfDay))
  (bind _daylength (Variables|Default|GetDayLength))
  (bind _returnvalue (/ _timeofday _daylength))
  (bind _returnvalue_2 (* _returnvalue 3.6e+02))
  (Transformation|SetActorRotation (Variables|Default|GetSunLight_Ref) (Math|Rotator|MakeRotator 0.0 (- _returnvalue_2 9e+01) -45.0))
  (Transformation|SetActorRotation (Variables|Default|GetMoonLight_Ref) (Math|Rotator|MakeRotator 0.0 (+ _returnvalue_2 9e+01) -45.0)))

(event Custom|CheckForMoon
  (bind _sunlight_ref (Variables|Default|GetSunLight_Ref))
  (bind _timeofday (Variables|Default|GetTimeOfDay))
  (bind _timeofday_2 (Variables|Default|GetTimeOfDay))
  (bind _moonlight_ref (Variables|Default|GetMoonLight_Ref))
  (bind _rootcomponent (Variables|/Script/Engine.Actor|GetRootComponent _sunlight_ref))
  (bind _lightcomponent (Variables|/Script/Engine.Light|GetLightComponent _moonlight_ref))
  (Utilities|FlowControl|Sequence
    (:then_0
      (if (and (> _timeofday 155.0) (< _timeofday 445.0))
        (Development|SetHiddeninGame _rootcomponent true false)
        (else
          (Development|SetHiddeninGame _rootcomponent false false))))
    (:then_1
      (if (and (> _timeofday_2 135.0) (< _timeofday_2 465.0))
        (Development|SetHiddeninGame _lightcomponent false false)
        (else
          (Development|SetHiddeninGame _lightcomponent true false))))))

(event EventTick
  (params (DeltaSeconds :type Float%20%28single-precision%29))
  (CallFunction|UpdateTimeOfDay))

(fn ConstructionScript)