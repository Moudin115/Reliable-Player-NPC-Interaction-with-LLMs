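; Procedural fence actor that picks one of six PCG fence graphs based on its FenceType value.
; On BeginPlay, a chain of integer checks assigns the matching graph to its PCG component through SetGraph.
; The choice happens only at runtime, since the construction script is empty, and values outside the handled range leave the component's graph unchanged.
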(event EventBeginPlay
  (bind _fencetype (Variables|Default|GetFenceType))
  ;[1 1 1] Fence Type Check
  (if (== _fencetype 0)
    ;[1 1 1] Fence Outcome
    (Class|PCGComponent|SetGraph (Variables|Default|GetPCG) "/Game/_mystuff/Procedural/PCG_Fence_0.PCG_Fence_0")
    (elif (== _fencetype 1)
      (Class|PCGComponent|SetGraph (Variables|Default|GetPCG) "/Game/_mystuff/Procedural/PCG_Fence_1.PCG_Fence_1")
      (elif (== _fencetype 2)
        (Class|PCGComponent|SetGraph (Variables|Default|GetPCG) "/Game/_mystuff/Procedural/PCG_Fence_2.PCG_Fence_2")
        (elif (== _fencetype 3)
          (Class|PCGComponent|SetGraph (Variables|Default|GetPCG) "/Game/_mystuff/Procedural/PCG_Fence_3.PCG_Fence_3")
          (elif (== _fencetype 4)
            (Class|PCGComponent|SetGraph (Variables|Default|GetPCG) "/Game/_mystuff/Procedural/PCG_Fence_4.PCG_Fence_4")
            (elif (== _fencetype 5)
              (Class|PCGComponent|SetGraph (Variables|Default|GetPCG) "/Game/_mystuff/Procedural/PCG_Fence_5.PCG_Fence_5"))))))))

(fn ConstructionScript)